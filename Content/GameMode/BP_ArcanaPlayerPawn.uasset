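; Player pawn for Arcana that acts as a mouse-driven spring-arm camera, snapped down onto the surface below it at BeginPlay.
; Mouse wheel drives a clamped zoom alpha, with curves setting arm length and pitch.
; Left-drag pans at a curve-scaled speed based on arm length; right-drag yaws with the cursor hidden, restoring its position on release.
; The two drags are mutually exclusive and suspend mouse-over events; GetIsRotating exposes rotation state.
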(event EventBeginPlay
  (bind _returnvalue (Transformation|GetActorLocation))
  ;[1 1 1] Move initial position down to surface
  (bind (_outhit _returnvalue_2) (Collision|LineTraceByChannel _returnvalue (- _returnvalue "0, 0,1000.000000") "TraceTypeQuery1" false 0 "None"))
  (if _returnvalue_2
    (Transformation|SetActorLocation (.Location (Collision|BreakHitResult _outhit)) false false)))

(event EventTick
  (params (DeltaSeconds :type Float%20%28single-precision%29))
  ;[1 1 1] Debug Draw
  (if (Variables|Default|GetbDebugDraw)
    (Rendering|Debug|DrawDebugSphere (Transformation|GetWorldLocation (Variables|Default|GetSpringArm)) 5e+01 12 "(R=1.000000,G=0.371560,B=0.000000,A=1.000000)" 0.0)))

(event Input|MouseEvents|MouseY
  (params (AxisValue :type Float%20%28single-precision%29))
  ;[1 1 1] Drag to move/rotate
  (if (Variables|Default|GetbLMBPressed)
    (Transformation|AddActorLocalOffset (Math|Vector|MakeVector (* AxisValue (Utilities|Time|GetWorldDeltaSeconds) -1.0 (Math|Curves|GetFloatValue (Variables|Default|GetDragSpeedCurve) (Variables|/Script/Engine.SpringArmComponent|GetTargetArmLength (Variables|Default|GetSpringArm)))) 0.0 0.0) false false)))

(event Input|MouseEvents|MouseWheelAxis
  (params (AxisValue :type Float%20%28single-precision%29))
  ;[1 1 1] Camera Zoom
  (bind _output_get (Variables|Default|SetZoomAlpha (Math|Float|Clamp(Float) (+ (* AxisValue (Utilities|Time|GetWorldDeltaSeconds) 3.5) (Variables|Default|GetZoomAlpha)))))
  (Variables|/Script/Engine.SpringArmComponent|SetTargetArmLength (Variables|Default|GetSpringArm) (Math|Curves|GetFloatValue (Variables|Default|GetCameraDistanceCurve) _output_get))
  (Transformation|SetRelativeRotation (Variables|Default|GetSpringArm) (Math|Rotator|MakeRotator 0.0 (* (Math|Curves|GetFloatValue (Variables|Default|GetCameraPitchCurve) (Variables|Default|GetZoomAlpha)) -1.0) 0.0) false false))

(event Input|MouseEvents|MouseX
  (params (AxisValue :type Float%20%28single-precision%29))
  ;[1 1 1] Drag to move/rotate
  (if (Variables|Default|GetbRMBPressed)
    (Class|Actor|AddActorWorldRotation (Math|Rotator|MakeRotator 0.0 0.0 (* AxisValue (Utilities|Time|GetWorldDeltaSeconds) 3.6e+02)))
    (elif (Variables|Default|GetbLMBPressed)
      (Transformation|AddActorLocalOffset (Math|Vector|MakeVector 0.0 (* AxisValue (Utilities|Time|GetWorldDeltaSeconds) -1.0 (Math|Curves|GetFloatValue (Variables|Default|GetDragSpeedCurve) (Variables|/Script/Engine.SpringArmComponent|GetTargetArmLength (Variables|Default|GetSpringArm)))) 0.0) false false))))

(event Input|MouseEvents|RightMouseButton
  (params (Key :type Key%20Structure :default "None"))
  (bind _returnvalue (Game|GetPlayerController 0))
  (bind _returnvalue_2 (Game|GetPlayerController 0))
  (bind (_locationx _locationy) (Game|Player|GetMousePosition _returnvalue))
  ;[1 1 1] Drag to move/rotate
  (:Pressed
    (if (not (Variables|Default|GetbLMBPressed))
      (Variables|Default|SetbRMBPressed true)
      (Variables|/Script/Engine.PlayerController|SetbShowMouseCursor _returnvalue false)
      (Variables|Default|SetMouseLocationX _locationx)
      (Variables|Default|SetMouseLocationY _locationy)
      (Input|SetInputModeGameOnly (Game|GetPlayerController 0))
      (Variables|/Script/Engine.PlayerController|SetbEnableMouseOverEvents _returnvalue_2 false)))
  (:Released
    (if (Variables|Default|GetbRMBPressed)
      (Variables|Default|SetbRMBPressed false)
      (Class|PlayerController|SetMouseLocation _returnvalue (Math|Float|Truncate (Variables|Default|GetMouseLocationX)) (Math|Float|Truncate (Variables|Default|GetMouseLocationY)))
      (Variables|/Script/Engine.PlayerController|SetbShowMouseCursor _returnvalue true)
      (Input|SetInputModeGameandUI (Game|GetPlayerController 0) 0 "LockOnCapture" false)
      (Variables|/Script/Engine.PlayerController|SetbEnableMouseOverEvents _returnvalue_2 true))))

(event Input|MouseEvents|LeftMouseButton
  (params (Key :type Key%20Structure :default "None"))
  (bind _returnvalue (Game|GetPlayerController 0))
  ;[1 1 1] Drag to move/rotate
  (:Pressed
    (if (not (Variables|Default|GetbRMBPressed))
      (Variables|Default|SetbLMBPressed true)
      (Variables|/Script/Engine.PlayerController|SetbEnableMouseOverEvents _returnvalue false)))
  (:Released
    (if (Variables|Default|GetbLMBPressed)
      (Variables|Default|SetbLMBPressed false)
      (Variables|/Script/Engine.PlayerController|SetbEnableMouseOverEvents _returnvalue true))))

(fn ConstructionScript)

(fn GetIsRotating
  (return (Variables|Default|GetbRMBPressed) (Variables|Default|GetMouseLocationX) (Variables|Default|GetMouseLocationY)))